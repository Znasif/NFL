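; BP_Spectator is a spectator character actor that gets randomized clothing colors for visual variety.
; Its Construction Script creates dynamic material instances for Torso and Legs, each taking a random palette color as primary and a random-hue variant as secondary.
; The random index never reaches the palette's last entry.
; A random body-mesh swap is present but disconnected, and the event graph holds only disabled stubs.
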(fn `UserConstructionScript`
  (bind _allclrs (`self.allclrs`))
  (bind _colr (`self.colr`))
  (bind _colr_2 (`self.colr`))
  (bind _allclrs_2 (`self.allclrs`))
  (`parent.UserConstructionScript`)
  (`|ExecutionSequence`
    (:`then_1`
      (bind _returnvalue (`KismetMaterialLibrary.CreateDynamicMaterialInstance` (`PrimitiveComponent.GetMaterial` (`self.Torso`) 0)))
      (set `self.colr` (`|GetArrayItem` _allclrs_2 (`KismetMathLibrary.RandomInteger` (- (`KismetArrayLibrary.Array_Length` _allclrs_2) 1))))
      (`MaterialInstanceDynamic.SetVectorParameterValue` _returnvalue "diffuse_color_1" _colr_2)
      (`KismetMathLibrary.LinearColor_SetRandomHue` _colr_2)
      (`MaterialInstanceDynamic.SetVectorParameterValue` _returnvalue "diffuse_color_2" _colr_2)
      (`PrimitiveComponent.SetMaterial` (`self.Torso`) 0 _returnvalue))
    (:`then_2`
      (bind _returnvalue_2 (`KismetMaterialLibrary.CreateDynamicMaterialInstance` (`PrimitiveComponent.GetMaterial` (`self.Legs`) 0)))
      (set `self.colr` (`|GetArrayItem` _allclrs (`KismetMathLibrary.RandomInteger` (- (`KismetArrayLibrary.Array_Length` _allclrs) 1))))
      (`MaterialInstanceDynamic.SetVectorParameterValue` _returnvalue_2 "diffuse_color_1" _colr)
      (`KismetMathLibrary.LinearColor_SetRandomHue` _colr)
      (`MaterialInstanceDynamic.SetVectorParameterValue` _returnvalue_2 "diffuse_color_2" _colr)
      (`PrimitiveComponent.SetMaterial` (`self.Legs`) 0 _returnvalue_2))))